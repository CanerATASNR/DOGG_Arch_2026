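; BP_CoinSpawner populates the level with coins and traps when play begins, using tagged actors as spawn points.
; Each "Coin" point has a roughly 40% chance to spawn a BP_Coin at its location and rotation.
; Every "Trap" point spawns a class picked at random from TrapList, using a freshly seeded random stream.
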(event `self.ReceiveBeginPlay`
  (bind _outactors (`GameplayStatics.GetAllActorsWithTag` "Coin"))
  (for _array_element _outactors
    (if (> (`KismetMathLibrary.RandomIntegerInRange` 0 100) 60)
      (bind (_returnvalue_location _returnvalue_rotation) (`KismetMathLibrary.BreakTransform` (`self.GetTransform` _array_element)))
      (`|SpawnActorFromClass` "/Game/Development/Blueprints/BP_Coin.BP_Coin_C" (`KismetMathLibrary.MakeTransform` _returnvalue_location _returnvalue_rotation) "Undefined" "MultiplyWithRoot" null null)))
  (bind _outactors_2 (`GameplayStatics.GetAllActorsWithTag` "Trap"))
  (for _array_element_2 _outactors_2
    (bind (_returnvalue_location_2 _returnvalue_rotation_2) (`KismetMathLibrary.BreakTransform` (`self.GetTransform` _array_element_2)))
    (`|SpawnActorFromClass` (`KismetArrayLibrary.Array_RandomFromStream` (`self.TrapList`) (`KismetMathLibrary.MakeRandomStream` (`KismetMathLibrary.RandomInteger` 2147483647))) (`KismetMathLibrary.MakeTransform` _returnvalue_location_2 _returnvalue_rotation_2) "Undefined" "MultiplyWithRoot" null null)))

(fn `UserConstructionScript`)