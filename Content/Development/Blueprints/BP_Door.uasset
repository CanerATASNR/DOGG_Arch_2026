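; BP_Door is a level exit that opens once all coins are collected and sends the player to the next level.
; On BeginPlay it finds the current level's row in DT_LevelList by matching level name.
; The first trigger destroys the door cube if no BP_Coin actors remain, otherwise logs a collect-coins message.
; The second trigger opens the level in the next numerically named row.
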(event `self.ReceiveBeginPlay`
  (bind _outrownames (`DataTableFunctionLibrary.GetDataTableRowNames` "/Game/Development/Data/DT_LevelList.DT_LevelList"))
  (for _array_element _outrownames
    (bind _returnvalue (`|GetDataTableRow` "/Game/Development/Data/DT_LevelList.DT_LevelList" _array_element)
      (:`then`
        (if (`KismetStringLibrary.EqualEqual_StrStr` (`.Reference_5_966C1247486AB652D157D2BA935EA2C4` (break `/Game/Development/Data/ST_Levels` _returnvalue)) (`KismetSystemLibrary.GetDisplayName` (`self.GetLevel`)))
          (set `self.CurrentLevel` _array_element))))))

(event `self.Box.OnComponentBeginOverlap`
  (params (OverlappedComponent :type "PrimitiveComponent Object Reference") (OtherActor :type "Actor Object Reference") (OtherComp :type "PrimitiveComponent Object Reference") (OtherBodyIndex :type Integer) (bFromSweep :type Boolean) (SweepResult :type "HitResult Structure (by ref)"))
  (if (== OtherActor (`GameplayStatics.GetPlayerCharacter` 0))
    (bind _outactors (`GameplayStatics.GetAllActorsOfClass` "/Game/Development/Blueprints/BP_Coin.BP_Coin_C"))
    (if (> (`KismetArrayLibrary.Array_Length` _outactors) 0)
      (`KismetSystemLibrary.LogString` "Paraları topla")
      (else
        (`ActorComponent.K2_DestroyComponent` (`self.Cube`))))))

(event `self.Box1.OnComponentBeginOverlap`
  (params (OverlappedComponent :type "PrimitiveComponent Object Reference") (OtherActor :type "Actor Object Reference") (OtherComp :type "PrimitiveComponent Object Reference") (OtherBodyIndex :type Integer) (bFromSweep :type Boolean) (SweepResult :type "HitResult Structure (by ref)"))
  (if (== OtherActor (`GameplayStatics.GetPlayerCharacter` 0))
    (bind _returnvalue (`|GetDataTableRow` "/Game/Development/Data/DT_LevelList.DT_LevelList" (`KismetStringLibrary.Conv_StringToName` (`KismetStringLibrary.Conv_IntToString` (+ (`KismetStringLibrary.Conv_StringToInt` (`KismetStringLibrary.Conv_NameToString` (`self.CurrentLevel`))) 1))))
      (:`then`
        (`GameplayStatics.OpenLevel` (`KismetStringLibrary.Conv_StringToName` (`.Reference_5_966C1247486AB652D157D2BA935EA2C4` (break `/Game/Development/Data/ST_Levels` _returnvalue))))))))

(fn `UserConstructionScript`)